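; TouchSwitchManager is a puzzle controller that links a group of touch switches to a set of moving blocks.
; On BeginPlay it tints every switch, block and block Niagara effect with a shared color through dynamic material instances and Niagara variables.
; Each Tick it polls the switches' active states, activating all blocks only when every switch is on and deactivating them otherwise.
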(event EventBeginPlay
  (bind _color (Variables|Default|GetColor))
  (Utilities|FlowControl|Sequence
    (:then_0
      (for _array_element (Variables|Default|GetTouchSwitches)
        (Utilities|Array|Add (Variables|Default|GetActivationStatuses) (Variables|/Game/Blueprints/TouchSwitch.TouchSwitch_C|GetIsActive _array_element))
        (bind _returnvalue (Rendering|Material|CreateDynamicMaterialInstance (Variables|/Script/Engine.StaticMeshActor|GetStaticMeshComponent _array_element) 0 (Rendering|Material|GetMaterial (Variables|/Script/Engine.StaticMeshActor|GetStaticMeshComponent _array_element) 0) "None" :!class /Script/Engine.PrimitiveComponent))
        (Rendering|Material|SetVectorParameterValue _returnvalue "Base Color" (Variables|Default|GetColor) :!class /Script/Engine.MaterialInstanceDynamic)))
    (:then_1
      (for _array_element_2 (Variables|Default|GetMovingBlocks)
        (bind _returnvalue_2 (Rendering|Material|CreateDynamicMaterialInstance (Variables|/Game/Blueprints/MovingBlock.MovingBlock_C|GetBlock _array_element_2) 0 (Rendering|Material|GetMaterial (Variables|/Game/Blueprints/MovingBlock.MovingBlock_C|GetBlock _array_element_2) 0) "None" :!class /Script/Engine.PrimitiveComponent))
        (Rendering|Material|SetVectorParameterValue _returnvalue_2 "Base Color" _color :!class /Script/Engine.MaterialInstanceDynamic)
        (Niagara|SetNiagaraVariable(LinearColor) (Variables|/Game/Blueprints/MovingBlock.MovingBlock_C|GetNiagara _array_element_2) "Color" _color)))))

(event Collision|EventActorBeginOverlap
  (params (OtherActor :type Actor%20Object%20Reference)))

(event EventTick
  (params (DeltaSeconds :type Float%20%28single-precision%29))
  (for (_array_element _array_index) (Variables|Default|GetTouchSwitches)
    (Utilities|Array|SetArrayElem (Variables|Default|GetActivationStatuses) _array_index (Variables|/Game/Blueprints/TouchSwitch.TouchSwitch_C|GetIsActive _array_element)))
  (if (Utilities|Array|ContainsItem (Variables|Default|GetActivationStatuses) false)
    (for _array_element_2 (Variables|Default|GetMovingBlocks)
      (Default|Deactivate _array_element_2))
    (else
      (for _array_element_3 (Variables|Default|GetMovingBlocks)
        (Default|Activate _array_element_3)))))

(fn ConstructionScript)