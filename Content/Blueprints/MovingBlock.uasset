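; Moving block actor that travels along a spline path, carrying its attached actors, and can be activated or deactivated.
; The MoveBlock timeline, rate-scaled by Speed over spline length, drives the block and restarts on closed loops; deactivation stops or reverses it.
; Each update re-captures attached actors' offsets from the block before moving them with it.
; A Niagara component receives the spline and loop flag at BeginPlay.
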(event Custom|Activate
  (bind _splinemovementpath (Variables|Default|GetSplineMovementPath))
  (Variables|Default|SetIsActive true)
  (bind _traveldistance (Timeline|MoveBlock Play)
    (:Update
      (CallFunction|UpdateBlockLocation (Spline|GetLocationatDistanceAlongSpline _splinemovementpath (* (Spline|GetSplineLength _splinemovementpath) _traveldistance) "World")))
    (:Finished
      (CallFunction|MovementEnd))))

(event Custom|Deactivate
  (bind _splinemovementpath (Variables|Default|GetSplineMovementPath))
  (Variables|Default|SetIsActive false)
  (if (Variables|Default|GetReverseWhenNotActive)
    (bind _traveldistance (Timeline|MoveBlock Reverse)
      (:Update
        (CallFunction|UpdateBlockLocation (Spline|GetLocationatDistanceAlongSpline _splinemovementpath (* (Spline|GetSplineLength _splinemovementpath) _traveldistance) "World")))
      (:Finished
        (CallFunction|MovementEnd)))
    (else
      (Timeline|MoveBlock Stop))))

(event Custom|MovementEnd
  (bind _splinemovementpath (Variables|Default|GetSplineMovementPath))
  (if (Variables|Default|GetClosedLoop)
    (if (and (Variables|Default|GetReverseWhenNotActive) (not (Variables|Default|GetIsActive)))
      (bind _traveldistance (Timeline|MoveBlock ReverseFromEnd)
        (:Update
          (CallFunction|UpdateBlockLocation (Spline|GetLocationatDistanceAlongSpline _splinemovementpath (* (Spline|GetSplineLength _splinemovementpath) _traveldistance) "World")))
        (:Finished
          (CallFunction|MovementEnd)))
      (else
        (Timeline|MoveBlock PlayFromStart)))))

(event EventBeginPlay
  (Utilities|FlowControl|Sequence
    (:then_0
      (Spline|SetClosedLoop (Variables|Default|GetSplineMovementPath) (Variables|Default|GetClosedLoop) true)
      (Components|Timeline|SetPlayRate (Variables|Default|GetMoveBlock) (/ (Variables|Default|GetSpeed) (Spline|GetSplineLength (Variables|Default|GetSplineMovementPath))))
      (Class|NiagaraComponent|SetVariableObject (Variables|Default|GetNiagara) "Spline" (Variables|Default|GetSplineMovementPath))
      (Class|NiagaraComponent|SetVariableBool (Variables|Default|GetNiagara) "ClosedLoop" (Variables|Default|GetClosedLoop))
      (CallFunction|SetOffsets))
    (:then_1
      (if (Variables|Default|GetIsActive)
        (CallFunction|Activate)))))

(event Collision|EventActorBeginOverlap
  (params (OtherActor :type Actor%20Object%20Reference)))

(event EventTick
  (params (DeltaSeconds :type Float%20%28single-precision%29)))

(fn ConstructionScript)

(fn SetOffsets
  (Utilities|Array|Clear (Variables|Default|GetAttachedActorOffsets))
  (for _array_element (Actor|GetAttachedActors true false)
    (Utilities|Array|Add (Variables|Default|GetAttachedActorOffsets) (- (Transformation|GetActorLocation _array_element) (Transformation|GetWorldLocation (Variables|Default|GetBlock))))))

(fn UpdateBlockLocation
  (params (NewLocation :type Vector))
  (CallFunction|SetOffsets)
  (Transformation|SetWorldLocation (Variables|Default|GetBlock) NewLocation false false)
  (for (_array_element _array_index) (Actor|GetAttachedActors true false)
    (Transformation|SetWorldLocation (Variables|/Script/Engine.Actor|GetRootComponent _array_element) (+ (Utilities|Array|Get(acopy) (Variables|Default|GetAttachedActorOffsets) _array_index) NewLocation) false false)))