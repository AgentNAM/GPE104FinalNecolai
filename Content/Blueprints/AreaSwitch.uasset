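; AreaSwitch is a trigger zone that switches IsActive on while enough qualifying objects are inside it.
; Overlap events run scale-sized sphere queries counting actors of listed classes, plus static mesh actors with a PhysicsKickable component.
; Reaching Minimum activates it once, with sound and higher material opacity; lower counts reset it.
; A count/minimum label follows the camera's rotation and takes the material's base color every Tick.
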(event EventBeginPlay
  (|CallParentFunction)
  (CallFunction|UpdateText))

(event Collision|EventActorBeginOverlap
  (params (OtherActor :type Actor%20Object%20Reference))
  (bind _staticmeshcomponent (Variables|Default|GetStaticMeshComponent))
  (bind _staticmeshcomponent_2 (Variables|Default|GetStaticMeshComponent))
  (CallFunction|UpdateText)
  (if (>= (CallFunction|CountOverlappingObjects) (Variables|Default|GetMinimum))
    (Utilities|FlowControl|DoOnce false :!label _label
      (:Completed
        (Variables|Default|SetIsActive true)
        (Audio|PlaySoundatLocation "/Engine/VREditor/Sounds/UI/Camera_Shutter.Camera_Shutter" (Transformation|GetActorLocation) "0, 0, 0" 1.0 1.0 0.0 0 0 0 0)
        (bind _returnvalue (Rendering|Material|CreateDynamicMaterialInstance _staticmeshcomponent 0 (Rendering|Material|GetMaterial _staticmeshcomponent 0) "None" :!class /Script/Engine.PrimitiveComponent))
        (Rendering|Material|SetScalarParameterValue _returnvalue "OpacityFill" 0.75 :!class /Script/Engine.MaterialInstanceDynamic)))
    (else
      (Utilities|FlowControl|Sequence
        (:then_0
          (goto _label Reset))
        (:then_1
          (Variables|Default|SetIsActive false)
          (Audio|PlaySoundatLocation "/Engine/VREditor/Sounds/VR_click1.VR_click1" (Transformation|GetActorLocation) "0, 0, 0" 1.0 1.0 0.0 0 0 0 0)
          (bind _returnvalue_2 (Rendering|Material|CreateDynamicMaterialInstance _staticmeshcomponent_2 0 (Rendering|Material|GetMaterial _staticmeshcomponent_2 0) "None" :!class /Script/Engine.PrimitiveComponent))
          (Rendering|Material|SetScalarParameterValue _returnvalue_2 "OpacityFill" 0.05 :!class /Script/Engine.MaterialInstanceDynamic))))))

(event EventTick
  (params (DeltaSeconds :type Float%20%28single-precision%29))
  (bind _staticmeshcomponent (Variables|Default|GetStaticMeshComponent))
  (bind _textrender (Variables|Default|GetTextRender))
  (|CallParentFunction DeltaSeconds)
  (Transformation|SetWorldRotation _textrender (Camera|GetCameraRotation (Game|GetPlayerCameraManager 0)) false false)
  (Transformation|AddLocalRotation _textrender "0.000000,180.000000,0.000000" false false)
  (bind _returnvalue (Rendering|Material|CreateDynamicMaterialInstance _staticmeshcomponent 0 (Rendering|Material|GetMaterial _staticmeshcomponent 0) "None" :!class /Script/Engine.PrimitiveComponent))
  (bind _returnvalue_2 (Rendering|Material|GetVectorParameterValue _returnvalue "Base Color" :!class /Script/Engine.MaterialInstanceDynamic))
  (Rendering|Components|TextRender|SetTextRenderColor (Variables|Default|GetTextRender) (Math|Conversions|ToColor(LinearColor) _returnvalue_2)))

(event Collision|EventActorEndOverlap
  (params (OtherActor :type Actor%20Object%20Reference))
  (bind _staticmeshcomponent (Variables|Default|GetStaticMeshComponent))
  (bind _staticmeshcomponent_2 (Variables|Default|GetStaticMeshComponent))
  (CallFunction|UpdateText)
  (if (>= (CallFunction|CountOverlappingObjects) (Variables|Default|GetMinimum))
    (Utilities|FlowControl|DoOnce false :!label _label
      (:Completed
        (Variables|Default|SetIsActive true)
        (Audio|PlaySoundatLocation "/Engine/VREditor/Sounds/UI/Camera_Shutter.Camera_Shutter" (Transformation|GetActorLocation) "0, 0, 0" 1.0 1.0 0.0 0 0 0 0)
        (bind _returnvalue (Rendering|Material|CreateDynamicMaterialInstance _staticmeshcomponent 0 (Rendering|Material|GetMaterial _staticmeshcomponent 0) "None" :!class /Script/Engine.PrimitiveComponent))
        (Rendering|Material|SetScalarParameterValue _returnvalue "OpacityFill" 0.75 :!class /Script/Engine.MaterialInstanceDynamic)))
    (else
      (Utilities|FlowControl|Sequence
        (:then_0
          (goto _label Reset))
        (:then_1
          (Variables|Default|SetIsActive false)
          (Audio|PlaySoundatLocation "/Engine/VREditor/Sounds/VR_click1.VR_click1" (Transformation|GetActorLocation) "0, 0, 0" 1.0 1.0 0.0 0 0 0 0)
          (bind _returnvalue_2 (Rendering|Material|CreateDynamicMaterialInstance _staticmeshcomponent_2 0 (Rendering|Material|GetMaterial _staticmeshcomponent_2 0) "None" :!class /Script/Engine.PrimitiveComponent))
          (Rendering|Material|SetScalarParameterValue _returnvalue_2 "OpacityFill" 0.05 :!class /Script/Engine.MaterialInstanceDynamic))))))

(fn ConstructionScript
  (|CallParentFunction))

(fn CountOverlappingObjects
  (bind _returnvalue (Transformation|GetActorLocation))
  (bind _returnvalue_2 (Transformation|GetActorScale3D))
  (bind _object_types (Variables|Default|GetObject%20Types))
  (bind _returnvalue_3 (* (.x _returnvalue_2) 5e+01))
  (for _array_element (Variables|Default|GetClasses)
    (bind _outactors (Collision|SphereOverlapActors _returnvalue _returnvalue_3 _object_types _array_element))
    (LocalVariables|SetOverlapping%20Objects (+ (LocalVariables|GetOverlapping%20Objects) (Utilities|Array|Length _outactors))))
  (bind _outactors_2 (Collision|SphereOverlapActors _returnvalue _returnvalue_3 _object_types "/Script/Engine.StaticMeshActor"))
  (for _array_element_2 _outactors_2
    (Utilities|IsValid (Actor|GetComponentbyClass _array_element_2 "/Game/Blueprints/Components/PhysicsKickable.PhysicsKickable_C")
      (:Is%20Valid
        (Math|Integer|IncrementInt (LocalVariables|GetOverlapping%20Objects)))))
  (return (LocalVariables|GetOverlapping%20Objects)))

(fn UpdateText
  (Rendering|Components|TextRender|SetText (Variables|Default|GetTextRender) (Utilities|Text|ToText(String) (Utilities|String|Append (Utilities|String|ToString(Integer) (CallFunction|CountOverlappingObjects)) "/" (Utilities|String|ToString(Integer) (Variables|Default|GetMinimum))))))