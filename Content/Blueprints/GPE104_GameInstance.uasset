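; Game instance that manages level progression, per-level speedrun best times and their persistence across sessions.
; An ordered level-name list drives level loading and advancing, returning to MainMenu after the last level.
; Current index, furthest index and best times persist in a single save slot, loaded or created on init.
; Starting directly in a listed level deletes the save and restarts progress from that level's index.
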(event Custom|NextLevel
  (if (< (Variables|Default|GetCurrentLevelIndex) (Utilities|Array|LastIndex (Variables|Default|GetLevelNames)))
    (bind _result (Math|Integer|IncrementInt (Variables|Default|GetCurrentLevelIndex))
      (:%20%20
        (CallFunction|UpdateMaxLevelIndex)
        (Game|OpenLevel(byName) (Utilities|Array|Get(acopy) (Variables|Default|GetLevelNames) _result))
        (CallFunction|SaveProgress)))
    (else
      (Game|OpenLevel(byName) "MainMenu"))))

(event Custom|GetSave
  (bind _returnvalue (SaveGame|DoesSaveGameExist "Save1"))
  (if _returnvalue
    (bind _returnvalue_2 (SaveGame|LoadGamefromSlot "Save1"))
    (bind _assave (Utilities|Casting|CastToSave _returnvalue_2))
    (Variables|Default|SetSave _assave)
    (CallFunction|LoadSavedProgress)
    (else
      (bind _returnvalue_3 (SaveGame|CreateSaveGameObject "/Game/Blueprints/Save.Save_C"))
      (Variables|Default|SetSave _returnvalue_3)
      (SaveGame|SaveGametoSlot _returnvalue_3 "Save1")
      (CallFunction|SaveProgress))))

(event EventInit
  (bind _levelnames (Variables|Default|GetLevelNames))
  (Utilities|FlowControl|Sequence
    (:then_0
      (bind _returnvalue (Game|GetCurrentLevelName true))
      (if (Utilities|Array|ContainsItem _levelnames (Utilities|String|StringToName _returnvalue))
        (CallFunction|DeleteSavedProgress)
        (Variables|Default|SetCurrentLevelIndex (Utilities|Array|FindItem _levelnames (Utilities|String|StringToName _returnvalue)))
        (CallFunction|UpdateMaxLevelIndex)))
    (:then_1
      (Variables|Default|SetBestTimes (CallFunction|GetDefaultBestTimes)))
    (:then_2
      (CallFunction|GetSave))))

(fn ResetCurrentLevel
  (bind _returnvalue (Game|GetCurrentLevelName true))
  (Game|OpenLevel(byName) (Utilities|String|StringToName _returnvalue)))

(fn LoadLevelbyIndex
  (params (LevelIndex :type Integer))
  (bind _output_get (Variables|Default|SetCurrentLevelIndex LevelIndex))
  (Game|OpenLevel(byName) (Utilities|Array|Get(acopy) (Variables|Default|GetLevelNames) _output_get)))

(fn UpdateMaxLevelIndex
  (Variables|Default|SetMaxLevelIndex (Math|Integer|Max(Integer) (Variables|Default|GetCurrentLevelIndex) (Variables|Default|GetMaxLevelIndex))))

(fn SaveProgress
  (bind _save (Variables|Default|GetSave))
  (bind _returnvalue (SaveGame|DoesSaveGameExist "Save1"))
  (if _returnvalue
    (Variables|/Game/Blueprints/Save.Save_C|SetSavedCurrentLevelIndex _save (Variables|Default|GetCurrentLevelIndex))
    (Variables|/Game/Blueprints/Save.Save_C|SetSavedMaxLevelIndex _save (Variables|Default|GetMaxLevelIndex))
    (Variables|/Game/Blueprints/Save.Save_C|SetSavedBestTimes _save (Variables|Default|GetBestTimes))
    (SaveGame|SaveGametoSlot _save "Save1")))

(fn LoadSavedProgress
  (bind _save (Variables|Default|GetSave))
  (bind _returnvalue (SaveGame|DoesSaveGameExist "Save1"))
  (if _returnvalue
    (Variables|Default|SetCurrentLevelIndex (Variables|/Game/Blueprints/Save.Save_C|GetSavedCurrentLevelIndex _save))
    (Variables|Default|SetMaxLevelIndex (Variables|/Game/Blueprints/Save.Save_C|GetSavedMaxLevelIndex _save))
    (Variables|Default|SetBestTimes (Variables|/Game/Blueprints/Save.Save_C|GetSavedBestTimes _save))))

(fn DeleteSavedProgress
  (bind _save (Variables|Default|GetSave))
  (bind _returnvalue (SaveGame|DoesSaveGameExist "Save1"))
  (if _returnvalue
    (bind _output_get (Variables|Default|SetCurrentLevelIndex 0))
    (Variables|/Game/Blueprints/Save.Save_C|SetSavedCurrentLevelIndex _save _output_get)
    (bind _output_get_2 (Variables|Default|SetMaxLevelIndex 0))
    (Variables|/Game/Blueprints/Save.Save_C|SetSavedMaxLevelIndex _save _output_get_2)
    (bind _output_get_3 (Variables|Default|SetBestTimes (CallFunction|GetDefaultBestTimes)))
    (Variables|/Game/Blueprints/Save.Save_C|SetSavedBestTimes _save _output_get_3)
    (SaveGame|DeleteGameinSlot "Save1")))

(fn RecordBestTime
  (params (NewTime :type Float%20%28double-precision%29))
  (bind _currentlevelindex (Variables|Default|GetCurrentLevelIndex))
  (bind _besttimes (Variables|Default|GetBestTimes))
  (bind _output (Utilities|Array|Get(acopy) _besttimes _currentlevelindex))
  (if (Variables|Default|GetSpeedrunMode)
    (if (or (< _output 0.0) (> _output NewTime))
      (Utilities|Array|SetArrayElem _besttimes _currentlevelindex NewTime))))

(fn GetDefaultBestTimes
  (bind _tempbesttimes (LocalVariables|GetTempBestTimes))
  (for _index (range 0 (Utilities|Array|LastIndex (Variables|Default|GetLevelNames)))
    (Utilities|Array|Add _tempbesttimes -1.0))
  (return _tempbesttimes))