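; Level goal actor that ends the level when the third-person character first overlaps it.
; A looping timer randomizes the hue of its cubes, light rays and point light, plus the spin rates that Tick applies.
; Overlap stops the speedrun timer, plays a sound, shows a random victory message and disables kicking.
; A timeline drives scale, light and global time dilation, compensating its play rate for the dilation, then loads the next level.
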(event Custom|Randomize
  (bind _rotationamountsrays (Variables|Default|GetRotationAmountsRays))
  (CallFunction|SetColor (Class|KismetMathLibrary|HSVtoRGB (Math|Random|RandomFloatinRange 0.0 3.6e+02) 1.0 1.0 1.0))
  (Variables|Default|SetRotationAmountOuter (Math|Random|RandomRotator false))
  (Variables|Default|SetRotationAmountInner (Math|Random|RandomRotator false))
  (for (_ _array_index) _rotationamountsrays
    (Utilities|Array|SetArrayElem _rotationamountsrays _array_index (Math|Random|RandomRotator false))))

(event EventBeginPlay
  (for _array_element (Components|GetChildrenComponents (Variables|Default|GetLightRays) false)
    (Transformation|SetWorldRotation _array_element (Math|Random|RandomRotator false) false false)
    (Utilities|Array|Add (Variables|Default|GetRotationAmountsRays) (Math|Random|RandomRotator false)))
  (CallFunction|Randomize)
  (Utilities|Time|SetTimerbyEvent (delegate Custom|Randomize) 0.25 true))

(event Collision|EventActorBeginOverlap
  (params (OtherActor :type Actor%20Object%20Reference))
  (bind _asbp_third_person_character (Utilities|Casting|CastToBP_ThirdPersonCharacter OtherActor))
  (Utilities|FlowControl|DoOnce false
    (:Completed
      (Default|StopSpeedrunTimer _asbp_third_person_character)
      (Audio|PlaySoundatLocation "/Engine/EditorSounds/Notifications/CompileFailed.CompileFailed" (Transformation|GetActorLocation) "0, 0, 0" 1.0 1.0 0.0 0 0 0 0)
      (bind _returnvalue (UserInterface|CreateWidget "/Game/Widgets/VictoryMessage.VictoryMessage_C"))
      (Default|SetRandomVictoryMessage _returnvalue)
      (UserInterface|Viewport|AddtoViewport _returnvalue 0)
      (bind (_direction _scale _timedilation _lightintensity) (Timeline|VictoryAnim PlayFromStart)
        (:Update
          (Utilities|FlowControl|Sequence
            (:then_0
              (Default|DisableKick _asbp_third_person_character))
            (:then_1
              (Transformation|SetActorScale3D _scale))
            (:then_2
              (Utilities|Time|SetGlobalTimeDilation _timedilation)
              (Components|Timeline|SetPlayRate (Variables|Default|GetVictoryAnim) (/ 1.0 (* _timedilation (Variables|Default|GetDuration)))))
            (:then_3
              (Rendering|Components|Light|SetIntensity (Variables|Default|GetPointLight) _lightintensity))))
        (:Finished
          (bind _asgpe104_game_instance (Utilities|Casting|CastToGPE104_GameInstance (Game|GetGameInstance)))
          (Default|NextLevel _asgpe104_game_instance))))))

(event EventTick
  (params (DeltaSeconds :type Float%20%28single-precision%29))
  (Utilities|FlowControl|Sequence
    (:then_0
      (Transformation|AddWorldRotation (Variables|Default|GetOuterCube) (* (Variables|Default|GetRotationAmountOuter) DeltaSeconds) false false))
    (:then_1
      (Transformation|AddWorldRotation (Variables|Default|GetInnerCube) (* (Variables|Default|GetRotationAmountInner) DeltaSeconds) false false))
    (:then_2
      (for (_array_element _array_index) (Components|GetChildrenComponents (Variables|Default|GetLightRays) false)
        (Transformation|AddWorldRotation _array_element (* (Utilities|Array|Get(acopy) (Variables|Default|GetRotationAmountsRays) _array_index) DeltaSeconds) false false)))))

(fn ConstructionScript)

(fn SetColor
  (params (Color :type Linear%20Color%20Structure))
  (Utilities|FlowControl|Sequence
    (:then_0
      (bind _returnvalue (Rendering|Material|CreateDynamicMaterialInstance (Variables|Default|GetOuterCube) 0 "/Game/Materials/M_Goal.M_Goal" "None" :!class /Script/Engine.PrimitiveComponent))
      (Rendering|Material|SetVectorParameterValue _returnvalue "Base Color" (Class|KismetMathLibrary|LinearColortoNewOpacity Color (Variables|Default|GetOpacityOuter)) :!class /Script/Engine.MaterialInstanceDynamic))
    (:then_1
      (bind _returnvalue_2 (Rendering|Material|CreateDynamicMaterialInstance (Variables|Default|GetInnerCube) 0 "/Game/Materials/M_Goal.M_Goal" "None" :!class /Script/Engine.PrimitiveComponent))
      (Rendering|Material|SetVectorParameterValue _returnvalue_2 "Base Color" (Class|KismetMathLibrary|LinearColortoNewOpacity Color (Variables|Default|GetOpacityInner)) :!class /Script/Engine.MaterialInstanceDynamic))
    (:then_2
      (for _array_element (Components|GetChildrenComponents (Variables|Default|GetLightRays) false)
        (bind _asprimitive_component (Utilities|Casting|CastToPrimitiveComponent _array_element))
        (bind _returnvalue_3 (Rendering|Material|CreateDynamicMaterialInstance _asprimitive_component 0 "/Game/Materials/M_Goal.M_Goal" "None" :!class /Script/Engine.PrimitiveComponent))
        (Rendering|Material|SetVectorParameterValue _returnvalue_3 "Base Color" (Class|KismetMathLibrary|LinearColortoNewOpacity Color (Variables|Default|GetOpacityRays)) :!class /Script/Engine.MaterialInstanceDynamic)))
    (:then_3
      (Rendering|Components|Light|SetLightColor (Variables|Default|GetPointLight) Color true))))