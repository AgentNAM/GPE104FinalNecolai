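; Breakable is an actor component that makes its owning actor shatter in an explosion effect when a player kicks it.
; It extends a parent's OnKicked event, calling the parent logic and then BreakSelf.
; BreakSelf spawns Blueprint_Effect_Explosion at the owner's transform with a short life span, then destroys the owner.
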(event EventBeginPlay
  (|CallParentFunction) ; This node is disabled and will not be called.\nDrag off pins to build functionality.
)

(event EventTick
  (params (DeltaSeconds :type Float%20%28single-precision%29))
  (|CallParentFunction DeltaSeconds) ; This node is disabled and will not be called.\nDrag off pins to build functionality.
)

(event EventOnKicked
  (params (Player :type BP%20Third%20Person%20Character%20Object%20Reference) (HitLocation :type Vector :default "0, 0, 0"))
  (|CallParentFunction Player HitLocation)
  (CallFunction|BreakSelf))

(fn BreakSelf
  (bind _returnvalue (Game|SpawnActorfromClass "/Game/StarterContent/Blueprints/Blueprint_Effect_Explosion.Blueprint_Effect_Explosion_C" (Transformation|GetActorTransform (Components|GetOwner)) "Undefined" "OverrideRootScale" 0 0))
  (Actor|SetLifeSpan _returnvalue 3.0)
  (Actor|DestroyActor (Components|GetOwner)))