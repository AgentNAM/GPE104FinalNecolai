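; Kickable component for static mesh actors that turns on physics and applies an impulse when a player kicks the owner.
; On begin play it sets the mesh material to show whether physics is already simulating.
; A kick switches to the simulating material and pushes along the normalized owner-to-player direction, scaled by ImpulseAmount.
; The impulse is applied at the player's location, and the supplied hit location only reaches the parent handler.
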(event EventBeginPlay
  (|CallParentFunction)
  (bind _asstatic_mesh_actor (Utilities|Casting|CastToStaticMeshActor (Components|GetOwner)))
  (if (Physics|IsSimulatingPhysics (Variables|/Script/Engine.StaticMeshActor|GetStaticMeshComponent _asstatic_mesh_actor) "None")
    (Rendering|Material|SetMaterial (Variables|/Script/Engine.StaticMeshActor|GetStaticMeshComponent _asstatic_mesh_actor) 0 (Variables|Default|GetMaterialSim))
    (else
      (Rendering|Material|SetMaterial (Variables|/Script/Engine.StaticMeshActor|GetStaticMeshComponent _asstatic_mesh_actor) 0 (Variables|Default|GetMaterialNoSim)))))

(event EventTick
  (params (DeltaSeconds :type Float%20%28single-precision%29))
  (|CallParentFunction DeltaSeconds) ; This node is disabled and will not be called.\nDrag off pins to build functionality.
)

(event EventOnKicked
  (params (Player :type BP%20Third%20Person%20Character%20Object%20Reference) (HitLocation :type Vector :default "0, 0, 0"))
  (bind _returnvalue (Components|GetOwner))
  (bind _returnvalue_2 (Transformation|GetActorLocation Player))
  (|CallParentFunction Player HitLocation)
  (bind _asstatic_mesh_actor (Utilities|Casting|CastToStaticMeshActor _returnvalue))
  (Physics|SetSimulatePhysics (Variables|/Script/Engine.StaticMeshActor|GetStaticMeshComponent _asstatic_mesh_actor) true)
  (Physics|AddImpulseatLocation (Variables|/Script/Engine.StaticMeshActor|GetStaticMeshComponent _asstatic_mesh_actor) (* (Math|Vector|Normalize (- _returnvalue_2 (Transformation|GetActorLocation _returnvalue))) (Variables|Default|GetImpulseAmount)) _returnvalue_2 "None")
  (Rendering|Material|SetMaterial (Variables|/Script/Engine.StaticMeshActor|GetStaticMeshComponent _asstatic_mesh_actor) 0 (Variables|Default|GetMaterialSim)))