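; TouchSwitch is a one-shot switch actor that activates when a qualifying actor overlaps it.
; An overlapping actor qualifies if its exact class is in the Classes list or it has a PhysicsKickable component.
; A DoOnce gate then latches IsActive, plays a camera shutter sound, and raises OpacityFill on a dynamic material instance of the static mesh, with no reset path.
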(event EventBeginPlay)

(event Collision|EventActorBeginOverlap
  (params (OtherActor :type Actor%20Object%20Reference))
  (bind _staticmeshcomponent (Variables|Debug|GetStaticMeshComponent))
  (if (or (Utilities|Array|ContainsItem (Variables|Default|GetClasses) (Utilities|GetClass OtherActor)) (Utilities|IsValid (Actor|GetComponentbyClass OtherActor "/Game/Blueprints/Components/PhysicsKickable.PhysicsKickable_C")))
    (Utilities|FlowControl|DoOnce false
      (:Completed
        (Variables|Default|SetIsActive true)
        (Audio|PlaySoundatLocation "/Engine/VREditor/Sounds/UI/Camera_Shutter.Camera_Shutter" (Transformation|GetActorLocation) "0, 0, 0" 1.0 1.0 0.0 0 0 0 0)
        (bind _returnvalue (Rendering|Material|CreateDynamicMaterialInstance _staticmeshcomponent 0 (Rendering|Material|GetMaterial _staticmeshcomponent 0) "None" :!class /Script/Engine.PrimitiveComponent))
        (Rendering|Material|SetScalarParameterValue _returnvalue "OpacityFill" 0.75 :!class /Script/Engine.MaterialInstanceDynamic)))))

(event EventTick
  (params (DeltaSeconds :type Float%20%28single-precision%29)))

(fn ConstructionScript)