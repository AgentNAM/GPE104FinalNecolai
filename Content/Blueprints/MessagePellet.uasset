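; A world pellet actor that reveals a text message while the third-person character overlaps it.
; On BeginPlay it sets the sphere's center opacity, then sizes the trigger after a short delay.
; Overlap hides the sphere, shows the text and spreads two cones in proportion to message length; leaving restores the idle look.
; Tick billboards the whole actor by copying the camera rotation plus a 180-degree turn.
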(event EventBeginPlay
  (bind _sphere (Variables|Default|GetSphere))
  (bind _returnvalue (Rendering|Material|CreateDynamicMaterialInstance _sphere 0 (Rendering|Material|GetMaterial _sphere 0) "None" :!class /Script/Engine.PrimitiveComponent))
  (Rendering|Material|SetScalarParameterValue _returnvalue "Opacity" (Variables|Default|GetCenterOpacity) :!class /Script/Engine.MaterialInstanceDynamic)
  (Utilities|FlowControl|Delay 0.1)
  (Components|Sphere|SetSphereRadius (Variables|Default|GetTriggerSphere) (Variables|Default|GetTriggerSphereRadius) true))

(event Collision|EventActorBeginOverlap
  (params (OtherActor :type Actor%20Object%20Reference))
  (bind _sphere (Variables|Default|GetSphere))
  (bind _conesoffsettext (Variables|Default|GetConesOffsetText))
  (bind _message (Variables|Default|GetMessage))
  (bind _conesoffsetbase (Variables|Default|GetConesOffsetBase))
  (bind _returnvalue (Utilities|String|ToString(Text) _message))
  (bind _returnvalue_2 (Utilities|String|ParseIntoArray _returnvalue " 
" false))
  (bind _returnvalue_3 (Utilities|Array|LastIndex _returnvalue_2))
  (bind _returnvalue_4 (* _conesoffsettext _returnvalue_3))
  (bind _returnvalue_5 (+ _returnvalue_4 _conesoffsetbase))
  (if (Class|GameplayStatics|ObjectIsA OtherActor "/Game/ThirdPerson/Blueprints/BP_ThirdPersonCharacter.BP_ThirdPersonCharacter_C")
    (bind _returnvalue_6 (Rendering|Material|CreateDynamicMaterialInstance _sphere 0 (Rendering|Material|GetMaterial _sphere 0) "None" :!class /Script/Engine.PrimitiveComponent))
    (Rendering|Material|SetScalarParameterValue _returnvalue_6 "Opacity" 0.0 :!class /Script/Engine.MaterialInstanceDynamic)
    (Rendering|Components|TextRender|SetText (Variables|Default|GetTextRender) (Variables|Default|GetMessage))
    (Transformation|SetRelativeLocation (Variables|Default|GetConeU) _returnvalue_5 false false)
    (Transformation|SetRelativeLocation (Variables|Default|GetConeD) (Math|Vector|NegateVector _returnvalue_5) false false)))

(event EventTick
  (params (DeltaSeconds :type Float%20%28single-precision%29))
  (Transformation|SetActorRotation (Camera|GetCameraRotation (Game|GetPlayerCameraManager 0)))
  (Transformation|AddActorLocalRotation "0.000000,180.000000,0.000000" false false))

(event Collision|EventActorEndOverlap
  (params (OtherActor :type Actor%20Object%20Reference))
  (bind _conesoffsetbase (Variables|Default|GetConesOffsetBase))
  (bind _sphere (Variables|Default|GetSphere))
  (if (Class|GameplayStatics|ObjectIsA OtherActor "/Game/ThirdPerson/Blueprints/BP_ThirdPersonCharacter.BP_ThirdPersonCharacter_C")
    (bind _returnvalue (Rendering|Material|CreateDynamicMaterialInstance _sphere 0 (Rendering|Material|GetMaterial _sphere 0) "None" :!class /Script/Engine.PrimitiveComponent))
    (Rendering|Material|SetScalarParameterValue _returnvalue "Opacity" (Variables|Default|GetCenterOpacity) :!class /Script/Engine.MaterialInstanceDynamic)
    (Rendering|Components|TextRender|SetText (Variables|Default|GetTextRender) (Variables|Default|Get?))
    (Transformation|SetRelativeLocation (Variables|Default|GetConeU) _conesoffsetbase false false)
    (Transformation|SetRelativeLocation (Variables|Default|GetConeD) (Math|Vector|NegateVector _conesoffsetbase) false false)))

(fn ConstructionScript)