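; Enemy actor that homes in on the player pawn and breaks itself when it hits a non-Enemy actor carrying a Hazard component.
; Each Tick zeroes the mesh's physics velocity, then ChasePlayer does a swept move and look-at along axes masked by Restriction.
; Chase speed scales with distance to the player relative to MaxDistance.
; Any hit sets a physics velocity pushing the enemy away from the impact point.
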(event EventBeginPlay)

(event Collision|EventActorBeginOverlap
  (params (OtherActor :type Actor%20Object%20Reference)))

(event EventTick
  (params (DeltaSeconds :type Float%20%28single-precision%29))
  (Utilities|FlowControl|Sequence
    (:then_0
      (if true
        (Physics|SetPhysicsLinearVelocity (Variables|Debug|GetStaticMeshComponent) "0, 0, 0" false "None")))
    (:then_1
      (Utilities|IsValid (Game|Player|GetPlayerPawn 0)
        (:Is%20Valid
          (CallFunction|ChasePlayer DeltaSeconds))))))

(event Collision|EventHit
  (params (MyComp :type Primitive%20Component%20Object%20Reference) (Other :type Actor%20Object%20Reference) (OtherComp :type Primitive%20Component%20Object%20Reference) (bSelfMoved :type Boolean) (HitLocation :type Vector :default "0, 0, 0") (HitNormal :type Vector :default "0, 0, 0") (NormalImpulse :type Vector :default "0, 0, 0") (Hit :type Hit%20Result%20Structure%20%28by%20ref%29))
  (Utilities|FlowControl|Sequence
    (:then_0
      (Physics|SetPhysicsLinearVelocity (Variables|Debug|GetStaticMeshComponent) (* (Math|Vector|Normalize (- (Transformation|GetActorLocation) HitLocation)) (Variables|Default|GetPushSpeed)) false "None"))
    (:then_1
      (Utilities|IsValid Other
        (:Is%20Valid
          (Utilities|IsValid (Actor|GetComponentbyClass Other "/Game/Blueprints/Components/Hazard.Hazard_C")
            (:Is%20Valid
              (if (not (Class|GameplayStatics|ObjectIsA Other "Enemy_C"))
                (Default|BreakSelf (Variables|Default|GetBreakable))))))))))

(fn ConstructionScript)

(fn ChasePlayer
  (params (B :type Float%20%28single-precision%29))
  (Transformation|SetActorLocationAndRotation (+ (Transformation|GetActorLocation) (* (* (Math|Vector|Normalize (- (Transformation|GetActorLocation (Game|Player|GetPlayerPawn 0)) (Transformation|GetActorLocation))) (Variables|Default|GetRestriction)) B (* (/ (Transformation|GetDistanceTo (Game|Player|GetPlayerPawn 0)) (Variables|Default|GetMaxDistance)) (Variables|Default|GetSpeed)))) (Math|Rotator|FindLookatRotation (Transformation|GetActorLocation) (+ (* (Transformation|GetActorLocation (Game|Player|GetPlayerPawn 0)) (Variables|Default|GetRestriction)) (* (Transformation|GetActorLocation) (- "1.000000,1.000000,1.000000" (Variables|Default|GetRestriction))))) true))